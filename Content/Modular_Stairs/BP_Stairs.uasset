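; BP_Stairs is a generated dynamic mesh actor that builds modular staircases with Geometry Script.
; On rebuild it derives step dimensions from StaircaseTop and NumSteps, then appends the first flight.
; Each MoreStairs direction adds a landing and a rotated flight, advancing a running base point to chain sections.
; Non-floating stairs get support boxes under added flights, and box-projected UVs are applied last for the material.
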(event `self.OnRebuildGeneratedMesh`
  (params (TargetMesh :type "DynamicMesh Object Reference"))
  (bind _uv_scale (`self.UV Scale`))
  (bind (_staircase_top_x _staircase_top_y _staircase_top_z) (`KismetMathLibrary.BreakVector` (`self.Staircase Top`)))
  (set `self.Dynamic Mesh` TargetMesh)
  (`|ExecutionSequence`
    (:`then_0`
      ;[1 1 1] Create Initial Staircase
      (`self.Calculate Staircase Dimentions`)
      (`GeometryScriptLibrary_MeshPrimitiveFunctions.AppendLinearStairs` (`self.Dynamic Mesh`) (struct) (struct) (`self.Step Width`) (`self.Step Height`) (`self.Step Depth`) (`self.Num Steps`) (`self.Floating Staircase`) null)
      (set `self.Current Staircase Base` (`KismetMathLibrary.MakeVector` (+ _staircase_top_x _staircase_top_y) 0.0 _staircase_top_z)))
    (:`then_1`
      ;[1 1 1] Create Stair Sections As Requested
      (for _array_element (`self.More Stairs`)
        (`self.Create Landing`)
        (`self.Create Staircase` _array_element)))
    (:`then_2`
      ;[1 1 1] UV Box Projection For Material
      (`GeometryScriptLibrary_MeshUVFunctions.SetMeshUVsFromBoxProjection` (`self.Dynamic Mesh`) 0 (`KismetMathLibrary.MakeTransform` (0.0 0.0 0.0) (struct) (`KismetMathLibrary.MakeVector` _uv_scale _uv_scale _uv_scale)) (struct) 2 null))))

(fn `Calculate Staircase Dimentions`
  (bind (_staircase_top_x _staircase_top_y _staircase_top_z) (`KismetMathLibrary.BreakVector` (`self.Staircase Top`)))
  (bind _num_steps (`self.Num Steps`))
  ;[1 1 1] Calculate Dimentions
  (bind _output_get (set `self.Staircase Lenght` _staircase_top_x))
  (bind _output_get_2 (set `self.Staircase Hight` _staircase_top_z))
  (set `self.Step Height` (/ _output_get_2 _num_steps))
  (set `self.Step Width` (* _staircase_top_y 2.0))
  (set `self.Step Depth` (/ _output_get _num_steps)))

(fn `Create Landing`
  (bind (_current_staircase_base_x _current_staircase_base_y _current_staircase_base_z) (`KismetMathLibrary.BreakVector` (`self.Current Staircase Base`)))
  (bind _step_width (`self.Step Width`))
  (`GeometryScriptLibrary_MeshPrimitiveFunctions.AppendBox` (`self.Dynamic Mesh`) (struct) (`KismetMathLibrary.MakeTransform` (`KismetMathLibrary.MakeVector` _current_staircase_base_x _current_staircase_base_y)) _step_width _step_width _current_staircase_base_z 0 0 0 "Base" null))

(fn `Create Staircase`
  (params (`Staircase Direction` :type "/Game/Modular_Stairs/E_Stair_Direction Enum" :default "NewEnumerator0"))
  (locals (`Staircase Rotation` :type "Float (double-precision)"))
  (bind (_current_staircase_base_x _current_staircase_base_y _current_staircase_base_z) (`KismetMathLibrary.BreakVector` (`self.Current Staircase Base`)))
  (bind (_current_staircase_base_x_2 _current_staircase_base_y_2 _current_staircase_base_z_2) (`KismetMathLibrary.BreakVector` (`self.Current Staircase Base`)))
  (bind (_staircase_top_x _staircase_top_y) (`KismetMathLibrary.BreakVector` (`self.Staircase Top`)))
  (bind (_current_staircase_base_x_3 _current_staircase_base_y_3 _current_staircase_base_z_3) (`KismetMathLibrary.BreakVector` (`self.Current Staircase Base`)))
  (bind (_staircase_top_x_2 _staircase_top_y_2) (`KismetMathLibrary.BreakVector` (`self.Staircase Top`)))
  (set `local.Staircase Rotation` (select `/Game/Modular_Stairs/E_Stair_Direction` `Staircase Direction` :`NewEnumerator1` 90.0 :`NewEnumerator2` 180.0 :`NewEnumerator3` 270.0))
  (`|ExecutionSequence`
    (:`then_0`
      ;[1 1 1] Create Staircase Section
      (bind (_x_out _y_out) (`self.XY Adjustment` (`local.Staircase Direction`) _staircase_top_y_2 _current_staircase_base_x _current_staircase_base_y))
      (`GeometryScriptLibrary_MeshPrimitiveFunctions.AppendLinearStairs` (`self.Dynamic Mesh`) (struct) (`KismetMathLibrary.MakeTransform` (`KismetMathLibrary.MakeVector` _x_out _y_out _current_staircase_base_z) (`KismetMathLibrary.MakeRotator` 0.0 0.0 (`local.Staircase Rotation`))) (`self.Step Width`) (`self.Step Height`) (`self.Step Depth`) (`self.Num Steps`) (`self.Floating Staircase`) null))
    (:`then_1`
      ;[1 1 1] Create Base Platform For Stairs
      (if (not (`self.Floating Staircase`))
        (bind (_x_out_2 _y_out_2) (`self.XY Adjustment` (`local.Staircase Direction`) (+ (/ (`self.Staircase Lenght`) 2.0) _staircase_top_y) _current_staircase_base_x_2 _current_staircase_base_y_2))
        (`GeometryScriptLibrary_MeshPrimitiveFunctions.AppendBox` (`self.Dynamic Mesh`) (struct) (`KismetMathLibrary.MakeTransform` (`KismetMathLibrary.MakeVector` _x_out_2 _y_out_2) (`KismetMathLibrary.MakeRotator` 0.0 0.0 (`local.Staircase Rotation`))) (`self.Staircase Lenght`) (`self.Step Width`) _current_staircase_base_z_2 0 0 0 "Base" null)))
    (:`then_2`
      ;[1 1 1] Set New Base Stair Location
      (bind (_x_out_3 _y_out_3) (`self.XY Adjustment` (`local.Staircase Direction`) (+ (`self.Staircase Lenght`) (`self.Step Width`)) _current_staircase_base_x_3 _current_staircase_base_y_3))
      (set `self.Current Staircase Base` (`KismetMathLibrary.MakeVector` _x_out_3 _y_out_3 (+ _current_staircase_base_z_3 (`self.Staircase Hight`)))))))

(fn `UserConstructionScript`)

(fn `XY Adjustment`
  (params (`Staircase Direction` :type "/Game/Modular_Stairs/E_Stair_Direction Enum" :default "NewEnumerator0") (`Adjustment Amount` :type "Float (double-precision)") (`X in` :type "Float (double-precision)") (`Y in` :type "Float (double-precision)"))
  (returns (`X Out` :type "Float (double-precision)") (`Y Out` :type "Float (double-precision)"))
  (return (+ `X in` (* (select `/Game/Modular_Stairs/E_Stair_Direction` `Staircase Direction` :`NewEnumerator0` 1.0 :`NewEnumerator2` -1.0) `Adjustment Amount`)) (+ `Y in` (* `Adjustment Amount` (select `/Game/Modular_Stairs/E_Stair_Direction` `Staircase Direction` :`NewEnumerator1` 1.0 :`NewEnumerator3` -1.0)))))