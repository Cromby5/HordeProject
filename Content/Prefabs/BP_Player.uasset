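; Player pawn with custom velocity-based movement, sprint and a smoothed third-person orbit camera, driven by Enhanced Input.
; Move input accelerates relative to the camera, while Tick applies deceleration, a planar speed cap and swept movement.
; Look input sets orbit angles for a target offset the camera eases toward, with velocity-based drag, while facing the player.
; Moving transfers camera yaw to the actor, preserving the camera's world position to avoid a jump.
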(event `self.ReceiveBeginPlay`
  ;[1 1 1] Initialise Input
  (bind _asplayer_controller (cast `PlayerController` (`self.GetController`)))
  (bind _returnvalue (pcsubsystem `EnhancedInputLocalPlayerSubsystem` _asplayer_controller))
  (`/Engine/EditorBlueprintResources/StandardMacros.IsValid` _returnvalue
    (:`Is Valid`
      (`EnhancedInputSubsystemInterface.AddMappingContext` _returnvalue "/Game/Input/IMC_Player.IMC_Player" 0 (struct))
      ;[1 1 1] Set Camera Position
      (`self.findCameraTargetPos`)
      (`SceneComponent.K2_SetRelativeLocation` (`self.Camera`) (`self.cameraTargetPos`) false false))))

(event `self.ReceiveTick`
  (params (DeltaSeconds :type "Float (single-precision)"))
  (`|ExecutionSequence`
    (:`then_0`
      ;[1 1 1] Deceleration
      (set `self.velocity` (- (`self.velocity`) (* (`self.velocity`) (`self.deceleration`) (`GameplayStatics.GetWorldDeltaSeconds`))))
      ;[1 1 1] Velocity Limit
      (if (> (`KismetMathLibrary.VSizeXYSquared` (`self.velocity`)) (`KismetMathLibrary.Square` (`self.maxVelocity`)))
        (set `self.velocity` (* (`KismetMathLibrary.Vector_Normal2D` (`self.velocity`)) (`self.maxVelocity`))))
      ;[1 1 1] Apply Movement
      (`self.K2_SetActorLocation` (+ (`self.K2_GetActorLocation`) (* (`self.velocity`) (`GameplayStatics.GetWorldDeltaSeconds`))) true))
    (:`then_1`
      ;[1 1 1] Camera Drag
      (`SceneComponent.K2_SetWorldLocation` (`self.Camera`) (- (`SceneComponent.K2_GetComponentLocation` (`self.Camera`)) (* (`self.velocity`) (`self.cameraDrag`) (`GameplayStatics.GetWorldDeltaSeconds`))) false false)
      ;[1 1 1] Camera Movement
      (if (> (`KismetMathLibrary.Vector_DistanceSquared` (`SceneComponent.RelativeLocation` (`self.Camera`)) (`self.cameraTargetPos`)) 25.0)
        (`SceneComponent.K2_AddRelativeLocation` (`self.Camera`) (* (- (`self.cameraTargetPos`) (`SceneComponent.RelativeLocation` (`self.Camera`))) (`self.cameraMoveSpeed`) (`GameplayStatics.GetWorldDeltaSeconds`)) false false))
      ;[1 1 1] Camera Focus
      (`self.findCameraFocus`)
      (`SceneComponent.K2_SetWorldRotation` (`self.Camera`) (`KismetMathLibrary.FindLookAtRotation` (`SceneComponent.K2_GetComponentLocation` (`self.Camera`)) (`self.cameraFocus`)) false false))))

(event `EnhancedInput|/Game/Input/IA_Move`
  (params (ActionValue :type "Vector2D Structure") (ElapsedSeconds :type "Float (double-precision)") (TriggeredSeconds :type "Float (double-precision)") (InputAction :type "InputAction Object Reference" :default "/Game/Input/IA_Move.IA_Move"))
  (bind (_x _y) (`KismetMathLibrary.BreakVector2D` ActionValue))
  (:`Triggered`
    ;[1 1 1] Apply Acceleration
    (set `self.velocity` (+ (`self.velocity`) (* (`KismetMathLibrary.Vector_Normal2D` (`SceneComponent.GetRightVector` (`self.Camera`))) (`self.acceleration`) (`GameplayStatics.GetWorldDeltaSeconds`) _x) (* (`KismetMathLibrary.Vector_Normal2D` (`SceneComponent.GetForwardVector` (`self.Camera`))) (`self.acceleration`) (`GameplayStatics.GetWorldDeltaSeconds`) _y)))
    (if (!= (`self.cameraHorizAngle`) 0.0)
      ;[1 1 1] Save Camera Position
      (set `self.camerWorldPosTemp` (`SceneComponent.K2_GetComponentLocation` (`self.Camera`)))
      ;[1 1 1] Player Face Camera Direction
      (`self.K2_AddActorWorldRotation` (`KismetMathLibrary.MakeRotator` 0.0 0.0 (`self.cameraHorizAngle`)))
      ;[1 1 1] Reset Camera Rotation
      (set `self.cameraHorizAngle` 0.0)
      (`self.findCameraTargetPos`)
      ;[1 1 1] Reset Camera Position
      (`SceneComponent.K2_SetWorldLocation` (`self.Camera`) (`self.camerWorldPosTemp`) false false))))

(event `EnhancedInput|/Game/Input/IA_Look`
  (params (ActionValue :type "Vector2D Structure") (ElapsedSeconds :type "Float (double-precision)") (TriggeredSeconds :type "Float (double-precision)") (InputAction :type "InputAction Object Reference" :default "/Game/Input/IA_Look.IA_Look"))
  (bind (_x _y) (`KismetMathLibrary.BreakVector2D` ActionValue))
  (:`Triggered`
    ;[1 1 1] Read Camera Input
    (set `self.cameraHorizDelta` (* (`self.cameraSensitivity`) (`GameplayStatics.GetWorldDeltaSeconds`) _x))
    (set `self.cameraVertDelta` (* (`self.cameraSensitivity`) (`GameplayStatics.GetWorldDeltaSeconds`) _y))
    ;[1 1 1] Apply Camera Rotation
    (set `self.cameraVertAngle` (`KismetMathLibrary.FClamp` (+ (`self.cameraVertAngle`) (`self.cameraVertDelta`)) (* (`self.cameraVertLimit`) -1.0) (`self.cameraVertLimit`)))
    (set `self.cameraHorizAngle` (+ (`self.cameraHorizAngle`) (`self.cameraHorizDelta`)))
    ;[1 1 1] Calculate Camera Target Position
    (`self.findCameraTargetPos`)))

(event `EnhancedInput|/Game/Input/IA_Sprint`
  (params (ActionValue :type Boolean) (ElapsedSeconds :type "Float (double-precision)") (TriggeredSeconds :type "Float (double-precision)") (InputAction :type "InputAction Object Reference" :default "/Game/Input/IA_Sprint.IA_Sprint"))
  (:`Started`
    (bind _output_get (set `self.sprinting` ActionValue :!label _label))
    (if _output_get
      (set `self.maxVelocity` (* (`self.maxVelocity`) (`self.sprintSpeedMultiplier`)))
      (set `self.acceleration` (* (`self.acceleration`) (`self.sprintSpeedMultiplier`)))
      (else
        (set `self.maxVelocity` (/ (`self.maxVelocity`) (`self.sprintSpeedMultiplier`)))
        (set `self.acceleration` (/ (`self.acceleration`) (`self.sprintSpeedMultiplier`))))))
  (:`Completed`
    (goto _label)))

(fn `findCameraFocus`
  (set `self.cameraFocus` (+ (`SceneComponent.K2_GetComponentLocation` (`self.Cube`)) (`KismetMathLibrary.MakeVector` 0.0 0.0 (`self.BaseEyeHeight`)))))

(fn `findCameraTargetPos`
  (set `self.cameraTargetPos` (`KismetMathLibrary.MakeVector` (* -1.0 (`KismetMathLibrary.DegCos` (`self.cameraHorizAngle`)) (`KismetMathLibrary.DegCos` (`self.cameraVertAngle`)) (`self.cameraDistance`)) (* -1.0 (`KismetMathLibrary.DegSin` (`self.cameraHorizAngle`)) (`KismetMathLibrary.DegCos` (`self.cameraVertAngle`)) (`self.cameraDistance`)) (+ (* -1.0 (`KismetMathLibrary.DegSin` (`self.cameraVertAngle`)) (`self.cameraDistance`)) (`self.BaseEyeHeight`)))))

(fn `UserConstructionScript`)